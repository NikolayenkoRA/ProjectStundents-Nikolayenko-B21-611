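; BP_Generator is the brick field of an Arkanoid-style game, with each brick a static mesh component of a single actor.
; The construction script lays out an X by Y grid of these meshes, spaced by DistanceX and DistanceY truncated to whole units.
; On a hit, the struck component is destroyed and, 70% of the time, a BP_Buff spawns at the hit location.
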(event `self.ReceiveHit`
  (params (MyComp :type "PrimitiveComponent Object Reference") (Other :type "Actor Object Reference") (OtherComp :type "PrimitiveComponent Object Reference") (bSelfMoved :type Boolean) (HitLocation :type "Vector Structure") (HitNormal :type "Vector Structure") (NormalImpulse :type "Vector Structure") (Hit :type "HitResult Structure (by ref)"))
  (`ActorComponent.K2_DestroyComponent` MyComp)
  (if (< (`KismetMathLibrary.RandomFloat`) 0.7)
    (`|SpawnActorFromClass` "/Game/MyLogic/Arcanoid/NewFolder/BP_Buff.BP_Buff_C" (`KismetMathLibrary.MakeTransform` HitLocation) "Undefined" "OverrideRootScale" null null)))

(fn `UserConstructionScript`
  (for _index (range (`self.x`))
    (for _index_2 (range (`self.y`))
      (`AddComponent|NODE_AddStaticMeshComponent-0` :`RelativeTransform` (`KismetMathLibrary.MakeTransform` (`KismetMathLibrary.MakeVector` (`KismetMathLibrary.Conv_IntToDouble` (* _index (`KismetMathLibrary.FTrunc` (`self.Distance_x`)))) (`KismetMathLibrary.Conv_IntToDouble` (* _index_2 (`KismetMathLibrary.FTrunc` (`self.Distance_y`))))))))))