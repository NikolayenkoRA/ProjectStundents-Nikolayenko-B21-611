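; BP_Ball is the ball for an Arcanoid-style game, bouncing off surfaces and scoring points.
; Each Tick it moves by Direction and Speed with a swept offset, then reflects Direction about the hit normal behind an always-true branch.
; When the hit actor's display name equals BP_Generator, it adds to its own Score and prints the total on screen.
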(event `self.ReceiveTick`
  (params (DeltaSeconds :type "Float (single-precision)"))
  (bind _sweephitresult (`self.K2_AddActorWorldOffset` (* (* (`self.direction`) (`self.speed`)) DeltaSeconds) true))
  (if true
    (bind (_bblockinghit _binitialoverlap _time _distance _location _impactpoint _normal _impactnormal _physmat _hitactor) (`GameplayStatics.BreakHitResult` _sweephitresult))
    (set `self.direction` (`KismetMathLibrary.GetReflectionVector` (`self.direction`) _normal))
    (if (`KismetStringLibrary.EqualEqual_StrStr` (`KismetSystemLibrary.GetDisplayName` _hitactor) "BP_Generator")
      (bind _output_get (set `self.Score` (+ (`self.Score`) 10)))
      (`KismetSystemLibrary.PrintString` (`KismetStringLibrary.Concat_StrStr` "Scroe:" (`KismetStringLibrary.Conv_IntToString` _output_get)) true true (struct :`R` 1.0 :`G` 0.012585 :`A` 1.0) 5.0))))

(fn `UserConstructionScript`)